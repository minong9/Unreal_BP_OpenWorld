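; Player character Blueprint that maps input to movement, camera look, target lock-on, dodge and weapon or skill selection.
; Combat is delegated to WeaponComponent, with mode switches gated on StateComponent's idle state.
; Tick smooths spring-arm zoom outside bow mode and, while grounded, feeds position plus three lagging trail points into a Material Parameter Collection for grass trampling.
; Also handles landing dust, footstep sound, test ragdoll and quitting after death.
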(event `InputAxis|MoveForward`
  (params (AxisValue :type "Float (single-precision)"))
  (`self.MoveForward` AxisValue))

(event `InputAxis|MoveRight`
  (params (AxisValue :type "Float (single-precision)"))
  (`self.MoveRight` AxisValue))

(event `InputAction|Walking`
  (params (Key :type "Key Structure"))
  (bind _charactermovement (`self.CharacterMovement`))
  (:`Pressed`
    (set `CharacterMovementComponent.MaxWalkSpeed` 400.0 _charactermovement))
  (:`Released`
    (set `CharacterMovementComponent.MaxWalkSpeed` 900.0 _charactermovement)))

(event `InputAxis|HorizontalLook`
  (params (AxisValue :type "Float (single-precision)"))
  (if (not (`/Game/Components/MovingComponent.IsFixedCamera` (`self.MovingComponent`)))
    (`self.AddControllerYawInput` AxisValue)))

(event `InputAxis|VerticalLook`
  (params (AxisValue :type "Float (single-precision)"))
  (if (not (`/Game/Components/MovingComponent.IsFixedCamera` (`self.MovingComponent`)))
    (`self.AddControllerPitchInput` AxisValue)))

(event `InputAction|Sword`
  (params (Key :type "Key Structure"))
  (:`Pressed`
    (if (`/Game/Components/StateComponent.IsIdleMode` (`self.StateComponent`))
      (`/Game/Components/WeaponComponent.SetSwordMode` (`self.WeaponComponent`)))))

(event `InputAction|Action`
  (params (Key :type "Key Structure"))
  (:`Pressed`
    (`/Game/Components/WeaponComponent.DoAction` (`self.WeaponComponent`))))

(event `InputAction|SubAction`
  (params (Key :type "Key Structure"))
  (:`Pressed`
    (`self.SubActionPressed`))
  (:`Released`
    (`self.SubActionReleased`)))

(event `InputAction|EButtonAction`
  (params (Key :type "Key Structure"))
  (:`Pressed`
    (`/Game/Components/WeaponComponent.EButtonAction` (`self.WeaponComponent`))))

(event `InputAction|GButtonAction`
  (params (Key :type "Key Structure"))
  (:`Pressed`
    (if (`/Game/Components/StateComponent.IsIdleMode` (`self.StateComponent`))
      (`/Game/Components/StateComponent.SetDodgeMode` (`self.StateComponent`)))))

(event `InputAction|RButtonAction`
  (params (Key :type "Key Structure"))
  (:`Pressed`
    (`/Game/Components/WeaponComponent.RButtonAction` (`self.WeaponComponent`))))

(event `InputAction|Ctrl_1ButtonAction`
  (params (Key :type "Key Structure"))
  (:`Pressed`
    (`/Game/Components/WeaponComponent.Ctrl_1_Action` (`self.WeaponComponent`))))

(event `InputAction|Bow`
  (params (Key :type "Key Structure"))
  (:`Pressed`
    (if (`/Game/Components/StateComponent.IsIdleMode` (`self.StateComponent`))
      (`/Game/Components/WeaponComponent.SetBowMode` (`self.WeaponComponent`)))))

(event `InputAction|Fist`
  (params (Key :type "Key Structure"))
  (:`Pressed`
    (if (`/Game/Components/StateComponent.IsIdleMode` (`self.StateComponent`))
      (`/Game/Components/WeaponComponent.SetFistMode` (`self.WeaponComponent`)))))

(event `InputAction|Hammer`
  (params (Key :type "Key Structure"))
  (:`Pressed`
    (if (`/Game/Components/StateComponent.IsIdleMode` (`self.StateComponent`))
      (`/Game/Components/WeaponComponent.SetHammerMode` (`self.WeaponComponent`)))))

(event `InputAction|Warp`
  (params (Key :type "Key Structure"))
  (:`Pressed`
    (if (`/Game/Components/StateComponent.IsIdleMode` (`self.StateComponent`))
      (`/Game/Components/WeaponComponent.SetWarpMode` (`self.WeaponComponent`)))))

(event `InputAction|Around`
  (params (Key :type "Key Structure"))
  (:`Pressed`
    (if (`/Game/Components/StateComponent.IsIdleMode` (`self.StateComponent`))
      (`/Game/Components/WeaponComponent.SetAroundMode` (`self.WeaponComponent`)))))

(event `InputAction|FireBall`
  (params (Key :type "Key Structure"))
  (:`Pressed`
    (if (`/Game/Components/StateComponent.IsIdleMode` (`self.StateComponent`))
      (`/Game/Components/WeaponComponent.SetFireBallMode` (`self.WeaponComponent`)))))

(event `InputAction|Ctrl_2ButtonAction`
  (params (Key :type "Key Structure"))
  (:`Pressed`
    (`/Game/Components/WeaponComponent.Ctrl_2_Action` (`self.WeaponComponent`))))

(event `InputAction|Targeting`
  (params (Key :type "Key Structure"))
  (:`Pressed`
    (`/Game/Components/TargetComponent.Toggle_Target` (`self.TargetComponent`))))

(event `InputAction|Left_Targeting`
  (params (Key :type "Key Structure"))
  (:`Pressed`
    (`/Game/Components/TargetComponent.ChangeFocus` (`self.TargetComponent`) false)))

(event `InputAction|Right_Targeting`
  (params (Key :type "Key Structure"))
  (:`Pressed`
    (`/Game/Components/TargetComponent.ChangeFocus` (`self.TargetComponent`) true)))

(event `Apply_Zoom`
  (bind _zooming (`self.Zooming`))
  (bind (_zoomdata_speed _zoomdata_minrange _zoomdata_maxrange _zoomdata_interpspeed) (break `/Game/BP/Human/Player/FZoomData` (`self.ZoomData`)))
  (bind _targetarmlength (`SpringArmComponent.TargetArmLength` (`self.SpringArm`)))
  (if (and (`self.IsNotBowMode`) (not (`KismetMathLibrary.NearlyEqual_FloatFloat` _targetarmlength _zooming 0.1)))
    (set `SpringArmComponent.TargetArmLength` (`KismetMathLibrary.FInterpTo` _targetarmlength _zooming (`GameplayStatics.GetWorldDeltaSeconds`) _zoomdata_interpspeed) (`self.SpringArm`))))

(event `InputAxis|Zoom`
  (params (AxisValue :type "Float (single-precision)"))
  (bind (_zoomdata_speed _zoomdata_minrange _zoomdata_maxrange) (break `/Game/BP/Human/Player/FZoomData` (`self.ZoomData`)))
  (if (`self.IsNotBowMode`)
    (set `self.Zooming` (`KismetMathLibrary.FClamp` (+ (`self.Zooming`) (* AxisValue _zoomdata_speed)) _zoomdata_minrange _zoomdata_maxrange))))

(event `self.ReceiveTick`
  (params (DeltaSeconds :type "Float (single-precision)"))
  (bind (_returnvalue_x _returnvalue_y _returnvalue_z) (`KismetMathLibrary.BreakVector` (`self.K2_GetActorLocation`)))
  (bind _returnvalue (- (`self.K2_GetActorLocation`) (`KismetMathLibrary.MakeVector` 0.0 0.0 (`CapsuleComponent.CapsuleHalfHeight` (`self.CapsuleComponent`)))))
  (`|ExecutionSequence`
    (:`then_0`
      (if (not (`NavMovementComponent.IsFalling` (`self.CharacterMovement`)))
        (`KismetMaterialLibrary.SetVectorParameterValue` "/Game/Materials/MP_Global.MP_Global" "PlayerPosition" (`KismetMathLibrary.Conv_VectorToLinearColor` _returnvalue))
        (bind _output_get (set `self.TP1` (`KismetMathLibrary.VLerp` (`self.TP1`) _returnvalue 0.5)))
        (`KismetMaterialLibrary.SetVectorParameterValue` "/Game/Materials/MP_Global.MP_Global" "Trampled Point1" (`KismetMathLibrary.Conv_VectorToLinearColor` _output_get))
        (bind _output_get_2 (set `self.TP2` (`KismetMathLibrary.VLerp` (`self.TP2`) _output_get 0.5)))
        (`KismetMaterialLibrary.SetVectorParameterValue` "/Game/Materials/MP_Global.MP_Global" "Trampled Point2" (`KismetMathLibrary.Conv_VectorToLinearColor` _output_get_2))
        (bind _output_get_3 (set `self.TP3` (`KismetMathLibrary.VLerp` (`self.TP3`) _output_get_2 0.5)))
        (`KismetMaterialLibrary.SetVectorParameterValue` "/Game/Materials/MP_Global.MP_Global" "Trampled Point3" (`KismetMathLibrary.Conv_VectorToLinearColor` _output_get_3))))
    (:`then_1`
      (`self.Apply_Zoom`))
    (:`then_2`
      (set `self.PrevZ_Position` _returnvalue_z))))

(event `self.ReceiveBeginPlay`
  (`parent.ReceiveBeginPlay`)
  (`|ExecutionSequence`
    (:`then_0`
      (`/Game/Components/MovingComponent.DisableControlRotation` (`self.MovingComponent`)))
    (:`then_1`
      (bind _asplayer_controller (cast `PlayerController` (`self.GetController`)))
      (bind _playercameramanager (`PlayerController.PlayerCameraManager` _asplayer_controller))
      (set `PlayerCameraManager.ViewPitchMin` -25.0 _playercameramanager)
      (set `PlayerCameraManager.ViewPitchMax` 40.0 _playercameramanager))
    (:`then_2`
      (set `self.Zooming` (`SpringArmComponent.TargetArmLength` (`self.SpringArm`))))))

(event `InputAction|TestKey`
  (params (Key :type "Key Structure"))
  (:`Pressed`
    (`self.Start Ragdoll`)))

(event `/Game/BP/BPI_Character.Footstep`
  (params (NewParam :type Boolean))
  (`GameplayStatics.PlaySoundAtLocation` "/Game/Sounds/Footsteps/CUE/Grass/Grass_Wander_Cue.Grass_Wander_Cue" (`self.K2_GetActorLocation`) (struct) 1.0 1.0 0.0 null null null))

(event `Dead`
  ;[1 1 1] Dead
  (`parent.Dead`)
  (`Controller.UnPossess` (`GameplayStatics.GetPlayerController` 0)))

(event `End_Dead`
  ;[1 1 1] Dead
  (`parent.End_Dead`)
  (`KismetSystemLibrary.QuitGame` null "Quit"))

(event `InputAction|Jumping`
  (params (Key :type "Key Structure"))
  ;[1 1 1] Jump / Land
  (:`Pressed`
    (`self.Jump`)
    (set `self.IsInAir` true))
  (:`Released`
    (`self.StopJumping`)))

(event `self.OnLanded`
  (params (Hit :type "HitResult Structure (by ref)"))
  ;[1 1 1] Jump / Land
  (`parent.OnLanded` Hit)
  (`GameplayStatics.SpawnEmitterAtLocation` "/Game/Effects/Jump_Dust.Jump_Dust" (- (`self.K2_GetActorLocation`) (`KismetMathLibrary.MakeVector` 0.0 0.0 (`CapsuleComponent.CapsuleHalfHeight` (`self.CapsuleComponent`)))) (struct) (10.0 10.0 10.0)))

(fn `IsNotBowMode`
  (returns (ReturnValue :type Boolean))
  (return (not (`/Game/Components/WeaponComponent.IsBowMode` (`self.WeaponComponent`)))))

(fn `IsNotGuardMode`
  (returns (ReturnValue :type Boolean))
  (return (not (`/Game/Components/StateComponent.IsGuardMode` (`self.StateComponent`)))))

(fn `UserConstructionScript`)