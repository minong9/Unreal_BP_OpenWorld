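; Master enemy AI human Blueprint that patrols, detects characters with a sphere overlap and chases living targets.
; Tick runs the current AIStateComponent state: random-yaw wandering, facing while equipping, distance-based chase or delayed return to idle.
; AI state changes set speed, detection and sword equip, while StateComponent changes pause or resume the AI.
; Close range sets Action mode, but the AI attack logic is unconnected; look, action and sword input handlers are also present.
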(event `self.ReceiveBeginPlay`
  ;[1 1 1] AI State Component : 뇌지컬이 바뀔때마다 호출되는 것임!
  (`parent.ReceiveBeginPlay`)
  (`|ExecutionSequence`
    (:`then_0`
      (add `/Game/Components/StateComponent.OnStateTypeChanged` (`self.StateComponent`) (delegate `OnStateTypeChanged`)))
    (:`then_1`
      (add `/Game/Components/AIStateComponent.OnAIStateChange` (`self.AIStateComponent`) (delegate `OnAIStateChange`)))))

(event `OnStateTypeChanged`
  (params (InPrevType :type "/Game/Components/EStateType Enum" :default "NewEnumerator0") (InNewType :type "/Game/Components/EStateType Enum" :default "NewEnumerator0"))
  ;[1 1 1] AI State Component : 뇌지컬이 바뀔때마다 호출되는 것임!
  (`parent.OnStateTypeChanged` InPrevType InNewType)
  (switch `/Game/Components/EStateType` InNewType
    (:`NewEnumerator0`
      (set `self.IsAIRunning` true))
    (:`NewEnumerator3`
      (`/Game/Components/MovingComponent.Stop` (`self.MovingComponent`)))
    (:`NewEnumerator4`
      (set `self.IsAIRunning` false))))

(event `InputAxis|HorizontalLook`
  (params (AxisValue :type "Float (single-precision)"))
  (`self.AddControllerYawInput` AxisValue))

(event `InputAxis|VerticalLook`
  (params (AxisValue :type "Float (single-precision)"))
  (`self.AddControllerPitchInput` AxisValue))

(event `InputAction|Sword`
  (params (Key :type "Key Structure"))
  (:`Pressed`
    (if (`/Game/Components/StateComponent.IsIdleMode` (`self.StateComponent`))
      (`/Game/Components/WeaponComponent.SetSwordMode` (`self.WeaponComponent`)))))

(event `InputAction|Action`
  (params (Key :type "Key Structure"))
  (:`Pressed`
    (`/Game/Components/WeaponComponent.DoAction` (`self.WeaponComponent`))))

(event `self.ReceiveTick`
  (params (DeltaSeconds :type "Float (single-precision)"))
  (if (`self.IsAIRunning`)
    (switch `/Game/Components/EAIStateType` (`/Game/Components/AIStateComponent.GetAIType` (`self.AIStateComponent`))
      (:`NewEnumerator0`
        (`self.Patrol`))
      (:`NewEnumerator2`
        (`self.SetYawRotation` (`self.K2_GetActorLocation` (`self.Target`))))
      (:`NewEnumerator3`
        (bind _target (`self.Target`)
          (:`then`
            (if (`/Game/Components/StateComponent.IsDeadMode` (`self.GetComponentByClass` _target "/Game/Components/StateComponent.StateComponent_C"))
              (`/Game/Components/AIStateComponent.SetWaitMode` (`self.AIStateComponent`) :!label _label)
              (else
                (`self.Trace`))))
          (:`else`
            (goto _label))))
      (:`NewEnumerator6`
        (`KismetSystemLibrary.Delay` 1.0)
        (`/Game/Components/AIStateComponent.SetIdleMode` (`self.AIStateComponent`))))))

(event `OnAIStateChange`
  (params (PrevType :type "/Game/Components/EAIStateType Enum" :default "NewEnumerator0") (NewType :type "/Game/Components/EAIStateType Enum" :default "NewEnumerator0"))
  (bind _movingcomponent (`self.MovingComponent`))
  ;[1 1 1] AI State Component : 뇌지컬이 바뀔때마다 호출되는 것임!
  (switch `/Game/Components/EAIStateType` NewType
    (:`NewEnumerator0`
      (`/Game/Components/MovingComponent.Move` _movingcomponent)
      (set `CharacterMovementComponent.MaxWalkSpeed` 400.0 (`self.CharacterMovement`))
      (set `self.Target` null)
      (`PrimitiveComponent.SetCollisionEnabled` (`self.Sphere`) "QueryOnly"))
    (:`NewEnumerator2`
      (`/Game/Components/WeaponComponent.SetSwordMode` (`self.WeaponComponent`)))
    (:`NewEnumerator3`
      (`/Game/Components/MovingComponent.Move` _movingcomponent)
      (set `CharacterMovementComponent.MaxWalkSpeed` 600.0 (`self.CharacterMovement`)))))

(event `Patrol`
  (bind (_returnvalue_roll _returnvalue_pitch _returnvalue_yaw) (`KismetMathLibrary.BreakRotator` (`KismetMathLibrary.RandomRotator` false)))
  ;[1 1 1] Patrol
  (set `self.CurTime` (+ (`GameplayStatics.GetWorldDeltaSeconds`) (`self.CurTime`)))
  (if (> (`self.CurTime`) (`self.Limit`))
    (`self.K2_SetActorRotation` (`KismetMathLibrary.MakeRotator` 0.0 0.0 _returnvalue_yaw))
    (set `self.CurTime` 0.0)
    (else
      (`self.MoveForward` 1.0))))

(event `Trace`
  ;[1 1 1] Trace
  (if (`/Game/Components/MovingComponent.IsCanMove` (`self.MovingComponent`))
    (`/Engine/EditorBlueprintResources/StandardMacros.IsValid` (`self.Target`)
      (:`Is Valid`
        (`self.UpdateDistance`)
        (if (<= (`self.PlayerToEnemyDistance`) 1100.0)
          (`|ExecutionSequence`
            (:`then_0`
              (`self.AddMovementInput` (`self.DirectionToPlayer`))
              (bind _target (`self.Target`)
                (:`then`
                  (`self.SetYawRotation` (`self.K2_GetActorLocation` _target)))
                (:`else`)))
            (:`then_1`
              (if (<= (`self.PlayerToEnemyDistance`) 150.0)
                (`/Game/Components/AIStateComponent.SetActionMode` (`self.AIStateComponent`)))))
          (else
            (`/Game/Components/AIStateComponent.SetWaitMode` (`self.AIStateComponent`))))))))

(event `self.Sphere.OnComponentBeginOverlap`
  (params (OverlappedComponent :type "PrimitiveComponent Object Reference") (OtherActor :type "Actor Object Reference") (OtherComp :type "PrimitiveComponent Object Reference") (OtherBodyIndex :type Integer) (bFromSweep :type Boolean) (SweepResult :type "HitResult Structure (by ref)"))
  (bind _aistatecomponent (`self.AIStateComponent`))
  ;[1 1 1] Collision
  (if (!= (`GameplayStatics.GetObjectClass` OtherActor) (`GameplayStatics.GetObjectClass` self))
    (bind _ascharacter (cast `Character` OtherActor))
    (if (not (`/Game/Components/StateComponent.IsDeadMode` (`self.GetComponentByClass` _ascharacter "/Game/Components/StateComponent.StateComponent_C")))
      (set `self.Target` _ascharacter)
      (`PrimitiveComponent.SetCollisionEnabled` (`self.Sphere`) "NoCollision")
      (if (`/Game/Components/WeaponComponent.IsUnamredMode` (`self.WeaponComponent`))
        (`/Game/Components/AIStateComponent.SetEquipMode` _aistatecomponent)
        (else
          (`/Game/Components/AIStateComponent.SetTraceMode` _aistatecomponent))))))

(event `Dead`
  ;[1 1 1] Dead
  (`parent.Dead`)
  (set `self.IsAIRunning` false))

(event `End_Dead`
  ;[1 1 1] Dead
  (`parent.End_Dead`))

(event `self.Hitted`
  (`parent.Hitted`))

(fn `SetYawRotation`
  (params (InLocation :type "Vector Structure"))
  (bind (_returnvalue_roll _returnvalue_pitch _returnvalue_yaw) (`KismetMathLibrary.BreakRotator` (`KismetMathLibrary.MakeRotFromX` (`KismetMathLibrary.Normal` (- (`self.K2_GetActorLocation` (`self.Target`)) (`self.K2_GetActorLocation` self))))))
  (`self.K2_SetActorRotation` (`KismetMathLibrary.MakeRotator` 0.0 0.0 _returnvalue_yaw)))

(fn `UpdateDistance`
  (bind _target (`self.Target`))
  (bind _returnvalue (- (`self.K2_GetActorLocation` _target) (`self.K2_GetActorLocation`)))
  (`/Engine/EditorBlueprintResources/StandardMacros.IsValid` _target
    (:`Is Valid`
      (set `self.PlayerToEnemyDistance` (`KismetMathLibrary.VSize` _returnvalue))
      (set `self.DirectionToPlayer` (`KismetMathLibrary.Normal` _returnvalue)))))

(fn `UserConstructionScript`)