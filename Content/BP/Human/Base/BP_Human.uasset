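; BP_Human is a base combat character that handles movement, health, hit reactions and death, delegating to State, Moving and Weapon components.
; Damaged and Guarded store hit data and enter Hitted state, whose change callback applies damage or triggers death.
; HitData drives montage, launch, effects, sound and camera shake, with body materials flashing red or blocking color.
; Hit stop briefly slows movable mesh actors through CustomTimeDilation, restored by timer.
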(event `MoveRight`
  (params (AxisValue :type "Float (double-precision)"))
  (bind (_returnvalue_roll _returnvalue_pitch _returnvalue_yaw) (`KismetMathLibrary.BreakRotator` (`self.GetControlRotation`)))
  (if (`/Game/Components/MovingComponent.IsCanMove` (`self.MovingComponent`))
    (`self.AddMovementInput` (`KismetMathLibrary.GetRightVector` (`KismetMathLibrary.MakeRotator` 0.0 0.0 _returnvalue_yaw)) AxisValue)))

(event `MoveForward`
  (params (AxisValue :type "Float (double-precision)"))
  (bind (_returnvalue_roll _returnvalue_pitch _returnvalue_yaw) (`KismetMathLibrary.BreakRotator` (`self.GetControlRotation`)))
  (if (`/Game/Components/MovingComponent.IsCanMove` (`self.MovingComponent`))
    (`self.AddMovementInput` (`KismetMathLibrary.GetForwardVector` (`KismetMathLibrary.MakeRotator` 0.0 0.0 _returnvalue_yaw)) AxisValue)))

(event `self.ReceiveBeginPlay`
  (for _array_element (`MeshComponent.GetMaterials` (`self.Mesh`))
    (bind _returnvalue (`KismetMaterialLibrary.CreateDynamicMaterialInstance` _array_element))
    (bind _returnvalue_2 (`KismetArrayLibrary.Array_Add` (`self.Materials`) _returnvalue))
    (`PrimitiveComponent.SetMaterial` (`self.Mesh`) _returnvalue_2 _returnvalue))
  (`|ExecutionSequence`
    (:`then_0`
      (set `self.Health` (`self.MaxHealth`))
      (add `/Game/Components/StateComponent.OnStateTypeChanged` (`self.StateComponent`) (delegate `OnStateTypeChanged`)))))

(event `/Game/IDamage.Damaged`
  (params (Attacker :type "Character Object Reference") (Causer :type "Actor Object Reference") (HitData :type "/Game/Weapons/FHitData Structure"))
  ;[1 1 1] Hitted
  (set `self.Attacker` Attacker)
  (set `self.Causer` Causer)
  (set `self.HitData` HitData)
  (`/Game/Components/StateComponent.SetHittedMode` (`self.StateComponent`)))

(event `/Game/IDamage.Guarded`
  (params (Attacker :type "Character Object Reference") (Causer :type "Actor Object Reference") (HitData :type "/Game/Weapons/FHitData Structure"))
  ;[1 1 1] Hitted
  (set `self.Attacker` Attacker)
  (set `self.Causer` Causer)
  (set `self.HitData` HitData)
  (`/Game/Components/StateComponent.SetHittedMode` (`self.StateComponent`)))

(event `OnStateTypeChanged`
  (params (InPrevType :type "/Game/Components/EStateType Enum" :default "NewEnumerator0") (InNewType :type "/Game/Components/EStateType Enum" :default "NewEnumerator0"))
  (`KismetSystemLibrary.PrintString` (`|GetEnumeratorNameAsString` InNewType))
  (switch `/Game/Components/EStateType` InNewType
    (:`NewEnumerator0`
      (`/Game/Components/MovingComponent.Move` (`self.MovingComponent`)))
    (:`NewEnumerator4`
      (`self.Hitted`)
      (switch `/Game/Components/EStateType` InPrevType
        (:`NewEnumerator8`
          (`/Game/Components/StateComponent.SetGuardMode` (`self.StateComponent`)))))
    (:`NewEnumerator6`
      (`self.Dead`))))

(event `Hitted`
  (bind _returnvalue (`self.K2_GetActorRotation`))
  (bind _returnvalue_2 (`self.K2_GetActorRotation`))
  (bind (_hitdata_damage _hitdata_montage _hitdata_playrate _hitdata_canmove _hitdata_launch _hitdata_launchrotator _hitdata_hitstop _hitdata_sound _hitdata_shakeclass _hitdata_effect _hitdata_effectlocation _hitdata_effectscale _hitdata_islaunchattacker _hitdata_niagaraeffect) (break `/Game/Weapons/FHitData` (`self.HitData`)))
  (bind (_hitdata_damage_2 _hitdata_montage_2 _hitdata_playrate_2 _hitdata_canmove_2 _hitdata_launch_2 _hitdata_launchrotator_2 _hitdata_hitstop_2 _hitdata_sound_2 _hitdata_shakeclass_2 _hitdata_effect_2 _hitdata_effectlocation_2 _hitdata_effectscale_2 _hitdata_islaunchattacker_2) (break `/Game/Weapons/FHitData` (`self.HitData`)))
  (bind (_hitdata_damage_3 _hitdata_montage_3 _hitdata_playrate_3 _hitdata_canmove_3 _hitdata_launch_3 _hitdata_launchrotator_3) (break `/Game/Weapons/FHitData` (`self.HitData`)))
  (bind (_hitdata_damage_4 _hitdata_montage_4 _hitdata_playrate_4 _hitdata_canmove_4 _hitdata_launch_4 _hitdata_launchrotator_4 _hitdata_hitstop_3) (break `/Game/Weapons/FHitData` (`self.HitData`)))
  (bind (_hitdata_damage_5 _hitdata_montage_5 _hitdata_playrate_5 _hitdata_canmove_5 _hitdata_launch_5 _hitdata_launchrotator_5 _hitdata_hitstop_4) (break `/Game/Weapons/FHitData` (`self.HitData`)))
  (bind (_hitdata_damage_6 _hitdata_montage_6 _hitdata_playrate_6 _hitdata_canmove_6 _hitdata_launch_6 _hitdata_launchrotator_6 _hitdata_hitstop_5 _hitdata_sound_3 _hitdata_shakeclass_3 _hitdata_effect_3 _hitdata_effectlocation_3 _hitdata_effectscale_3) (break `/Game/Weapons/FHitData` (`self.HitData`)))
  (bind (_damage _montage _playrate) (break `/Game/Weapons/FHitData` (`self.HitData`)))
  (bind (_damage_2 _montage_2 _playrate_2 _canmove _launch _launchrotator _hitstop _sound _shakeclass) (break `/Game/Weapons/FHitData` (`self.HitData`)))
  (bind (_returnvalue_x _returnvalue_y) (`KismetMathLibrary.BreakVector` (- (`self.K2_GetActorLocation`) (`self.K2_GetActorLocation` (`self.Attacker`)))))
  (bind (_returnvalue_roll _returnvalue_pitch _returnvalue_yaw) (`KismetMathLibrary.BreakRotator` (`KismetMathLibrary.MakeRotFromX` (`KismetMathLibrary.MakeVector` _returnvalue_x _returnvalue_y))))
  (bind _returnvalue_3 (* (`KismetMathLibrary.GetForwardVector` (`KismetMathLibrary.MakeRotator` (+ _returnvalue_roll (.roll _hitdata_launchrotator_3)) (+ _returnvalue_pitch (.pitch _hitdata_launchrotator_3)) (+ _returnvalue_yaw (.yaw _hitdata_launchrotator_3)))) _hitdata_launch_3))
  ;[1 1 1] Hitted
  (bind _output_get (set `self.Health` (`KismetMathLibrary.FClamp` (- (`self.Health`) (`.Damage_2_F9FD27D74040BB9E71099A847A8FF178` (break `/Game/Weapons/FHitData` (`self.HitData`)))) 0.0 (`self.MaxHealth`))))
  (if (<= _output_get 0.0)
    (`/Game/Components/StateComponent.SetDeadMode` (`self.StateComponent`))
    (else
      (`self.PlayAnimMontage` _montage _playrate)
      (`|ExecutionSequence`
        (:`then_0`
          (if (`KismetMathLibrary.NearlyEqual_FloatFloat` _damage)
            (for _array_element (`self.Materials`)
              (`MaterialInstanceDynamic.SetVectorParameterValue` _array_element "BodyColor" (struct :`R` 0.260417 :`G` 0.233243 :`B` 0.208333)))
            (`KismetSystemLibrary.Delay` 0.15)
            (for _array_element_2 (`self.Materials`)
              (if true
                (`MaterialInstanceDynamic.SetVectorParameterValue` _array_element_2 "BodyColor" (`self.BodyColor`))))
            (else
              (for _array_element_3 (`self.Materials`)
                (`MaterialInstanceDynamic.SetVectorParameterValue` _array_element_3 "BodyColor" (struct :`R` 1.0 :`A` 1.0)))
              (`KismetSystemLibrary.Delay` 0.15)
              (for _array_element_4 (`self.Materials`)
                (if true
                  (`MaterialInstanceDynamic.SetVectorParameterValue` _array_element_4 "BodyColor" (`self.BodyColor`))))))
          (bind _target (`self.Target`)
            (:`then`
              (bind (_returnvalue_roll_2 _returnvalue_pitch_2 _returnvalue_yaw_2) (`KismetMathLibrary.BreakRotator` (`KismetMathLibrary.FindLookAtRotation` (`self.K2_GetActorLocation`) (`self.K2_GetActorLocation` _target))))
              (`self.K2_SetActorRotation` (`KismetMathLibrary.MakeRotator` 0.0 0.0 _returnvalue_yaw_2))
              (`self.LaunchCharacter` _returnvalue_3 false true)
              (if _hitdata_islaunchattacker_2
                (`self.LaunchCharacter` (`self.Attacker`) (* _returnvalue_3 1.0) false true)))
            (:`else`)))
        (:`then_1`
          (`GameplayStatics.SpawnEmitterAtLocation` _hitdata_effect_3 (+ (`self.K2_GetActorLocation`) (`KismetMathLibrary.GreaterGreater_VectorRotator` _hitdata_effectlocation_3 _returnvalue_2)) _returnvalue_2 _hitdata_effectscale_3)
          (`NiagaraFunctionLibrary.SpawnSystemAtLocation` _hitdata_niagaraeffect (+ (`self.K2_GetActorLocation`) (`KismetMathLibrary.GreaterGreater_VectorRotator` _hitdata_effectlocation _returnvalue)) _returnvalue _hitdata_effectscale)
          (`GameplayStatics.SpawnSoundAtLocation` (`.Sound_19_D353130441EDA9F612CD3CA3BD730586` (break `/Game/Weapons/FHitData` (`self.HitData`))) (`self.K2_GetActorLocation`) (struct) 1.0 1.0 0.0 null null)
          (if (`KismetSystemLibrary.IsValidClass` _shakeclass)
            (`PlayerCameraManager.StartCameraShake` :`self` (`GameplayStatics.GetPlayerCameraManager` 0) :`ShakeClass` _shakeclass))
          (if (not (`KismetMathLibrary.NearlyEqual_FloatFloat` _hitdata_hitstop_3 0.0 1e-05))
            (bind _outactors (`GameplayStatics.GetAllActorsOfClass` "/Script/Engine.Actor"))
            (for _array_element_5 _outactors
              (bind _returnvalue_4 (`self.GetComponentByClass` _array_element_5 "/Script/Engine.MeshComponent"))
              (`/Engine/EditorBlueprintResources/StandardMacros.IsValid` _returnvalue_4
                (:`Is Valid`
                  (if (`|EnumEquality` (`SceneComponent.Mobility` _returnvalue_4) "Movable")
                    (`KismetArrayLibrary.Array_Add` (`self.Delation Actors`) _array_element_5)
                    (set `Actor.CustomTimeDilation` 0.05 _array_element_5)))))
            (`KismetSystemLibrary.K2_SetTimer` self "RestoreTimeDelation" _hitdata_hitstop_4)
            (`self.PlayHitStop_Exit`)))))))

(event `PlayHitStop_Exit`
  ;[1 1 1] Hitted
)

(event `RestoreTimeDelation`
  (bind _delation_actors (`self.Delation Actors`))
  ;[1 1 1] Hitted
  (for _array_element _delation_actors
    (set `Actor.CustomTimeDilation` 1.0 _array_element))
  (`KismetArrayLibrary.Array_Clear` _delation_actors))

(event `Dead`
  ;[1 1 1] Dead
  (`PrimitiveComponent.SetCollisionProfileName` (`self.CapsuleComponent`) "IgnorePawn" true)
  (`self.PlayAnimMontage` "/Game/Character/Montages/Enemy_DeadFall_Montage.Enemy_DeadFall_Montage"))

(event `End_Dead`
  ;[1 1 1] Dead
  (`/Game/Components/WeaponComponent.DestroyWeapon` (`self.WeaponComponent`))
  (`self.K2_DestroyActor`))

(event `self.OnLanded`
  (params (Hit :type "HitResult Structure (by ref)"))
  (`/Game/Components/WeaponComponent.InitCommand` (`self.WeaponComponent`)))

(fn `SubActionPressed`
  (if (`/Game/Components/StateComponent.IsIdleMode` (`self.StateComponent`))
    (`/Game/Components/WeaponComponent.SubActionPressed` (`self.WeaponComponent`))))

(fn `SubActionReleased`
  (if (not (`/Game/Components/StateComponent.IsEquipMode` (`self.StateComponent`)))
    (`/Game/Components/WeaponComponent.SubActionReleased` (`self.WeaponComponent`))))

(fn `UserConstructionScript`)