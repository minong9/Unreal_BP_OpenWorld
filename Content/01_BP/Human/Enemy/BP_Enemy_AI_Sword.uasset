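; BP_Enemy_AI_Sword is a sword enemy Blueprint whose only live logic here is a reaction to landing from a fall.
; After calling the parent landing handler, it checks vertical velocity, playing a rise montage for moderate falls and a katana knockdown-and-rise montage for hard ones.
; Other events are empty or disabled, and an unconnected fragment that would enable mesh physics simulation never runs.
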(event `self.CapsuleComponent.OnComponentBeginOverlap`
  (params (OverlappedComponent :type "PrimitiveComponent Object Reference") (OtherActor :type "Actor Object Reference") (OtherComp :type "PrimitiveComponent Object Reference") (OtherBodyIndex :type Integer) (bFromSweep :type Boolean) (SweepResult :type "HitResult Structure (by ref)")))

(event `self.OnLanded`
  (params (Hit :type "HitResult Structure (by ref)"))
  (bind (_velocity_x _velocity_y _velocity_z) (`KismetMathLibrary.BreakVector` (`MovementComponent.Velocity` (`self.CharacterMovement`))))
  (`parent.OnLanded` Hit)
  (if (> _velocity_z -500.0)
    _
    (elif (<= _velocity_z -2000.0)
      (`self.PlayAnimMontage` "/Game/02_Character/Montages/Common/Hit/Katana_Blade_KnockDownAndRise_Damage_Montage.Katana_Blade_KnockDownAndRise_Damage_Montage")
      (else
        (`self.PlayAnimMontage` "/Game/02_Character/Montages/Common/Hit/rise_Montage.rise_Montage")))))

(fn `UserConstructionScript`
  (`parent.UserConstructionScript`))