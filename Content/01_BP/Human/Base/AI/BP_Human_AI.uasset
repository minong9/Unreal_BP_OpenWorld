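; AI-driven human character Blueprint that links its state component to a BP_AIController.
; BeginPlay caches the controller and binds state changes, deactivating AI on Hitted or Dead; other combat overrides only call the parent.
; An older in-Blueprint patrol, trace and battle state machine with target detection remains unwired, leaving Patrol and Trace empty.
; Separate graphs still carry player look, attack and sword-equip input bindings.
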(event `InputAxis|HorizontalLook`
  (params (AxisValue :type "Float (single-precision)"))
  (`self.AddControllerYawInput` AxisValue))

(event `InputAxis|VerticalLook`
  (params (AxisValue :type "Float (single-precision)"))
  (`self.AddControllerPitchInput` AxisValue))

(event `InputAction|Sword`
  (params (Key :type "Key Structure"))
  (:`Pressed`
    (if (`/Game/03_Components/StateComponent.IsIdleMode` (`self.StateComponent`))
      (`/Game/03_Components/WeaponComponent.SetSwordMode` (`self.WeaponComponent`)))))

(event `InputAction|Action`
  (params (Key :type "Key Structure"))
  (:`Pressed`
    (`/Game/03_Components/WeaponComponent.DoAction` (`self.WeaponComponent`))))

(event `self.ReceiveBeginPlay`
  ;[0 0.2133 1] AI State Component : 뇌지컬이 바뀔때마다 호출되는 것임!
  (`parent.ReceiveBeginPlay`)
  (`|ExecutionSequence`
    (:`then_0`
      (add `/Game/03_Components/StateComponent.OnStateTypeChanged` (`self.StateComponent`) (delegate `OnStateTypeChanged`))
      (bind _asbp_aicontroller (cast `/Game/01_BP/Human/Base/AI/BP_AIController` (`AIBlueprintHelperLibrary.GetAIController` self)))
      (set `self.OwnController` _asbp_aicontroller))))

(event `OnStateTypeChanged`
  (params (InPrevType :type "/Game/03_Components/EStateType Enum" :default "NewEnumerator0") (InNewType :type "/Game/03_Components/EStateType Enum" :default "NewEnumerator0"))
  ;[0 0.2133 1] AI State Component : 뇌지컬이 바뀔때마다 호출되는 것임!
  (`parent.OnStateTypeChanged` InPrevType InNewType)
  (switch `/Game/03_Components/EStateType` InNewType
    (:`NewEnumerator4`
      _)
    (:`NewEnumerator6`
      _))
  (`/Game/01_BP/Human/Base/AI/BP_AIController.DeactiveAI` (`self.OwnController`)))

(event `Dead`
  ;[1 1 1] Dead
  (`parent.Dead`))

(event `self.Hitted`
  (`parent.Hitted`))

(event `End_Dead`
  ;[1 1 1] Dead
  (`parent.End_Dead`))

(event `Patrol`
  ;[1 1 1] Patrol
)

(event `self.OnLanded`
  (params (Hit :type "HitResult Structure (by ref)"))
  (`parent.OnLanded` Hit))

(event `/Game/IDamage.Parried`
  (params (Attacker :type "Character Object Reference") (Causer :type "Actor Object Reference"))
  (`parent.Parried` Attacker Causer))

(event `Trace`
  ;[1 1 1] Trace
)

(fn `ApplyLaunch`
  (`parent.ApplyLaunch`))

(fn `DodgeAction`
  (`parent.DodgeAction`))

(fn `UserConstructionScript`)