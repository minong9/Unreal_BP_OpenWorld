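; AI controller for the Aurora boss that runs the pawn's behavior tree on possess, takes its team ID, and stops logic on unpossess.
; Perception updates fill an empty blackboard Target with a BP_Human from another team.
; Tick keeps that target while known and alive, otherwise stops movement and assigns a living, known enemy, if any.
; ActiveAI and DeactiveAI switch the blackboard's StateOfBehavior enum.
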(event `self.ReceivePossess`
  (params (PossessedPawn :type "Pawn Object Reference"))
  (bind _asbp_boss_aurora (cast `/Game/01_BP/Boss/BP_Boss_Aurora` PossessedPawn))
  (set `self.OwnerTeamID` (`/Game/01_BP/Boss/BP_Boss_Aurora.TeamID` _asbp_boss_aurora))
  (bind _behaviortree (`/Game/01_BP/Boss/BP_Boss_Aurora.BehaviorTree` _asbp_boss_aurora)
    (:`then`
      (`self.RunBehaviorTree` _behaviortree) ; 이거 자체에 Use Black Board? 이게 포함되어 있음. 그래서 수행하면서 연결된 블랙보드를 자기자신에게 셋팅해둠
    )
    (:`else`)))

(event `self.ReceiveUnPossess`
  (params (UnpossessedPawn :type "Pawn Object Reference"))
  (bind _braincomponent (`self.BrainComponent`)
    (:`then`
      (`BrainComponent.StopLogic` _braincomponent "") ; 그래서 애초에 AIController에서 런 비헤이비어 트리를 시행할 때 가져온 블랙보드를 참조하여 그걸 틱에서 멈춤(업데이트 멈춤)
    )
    (:`else`)))

(event `self.ReceiveTick`
  (params (DeltaSeconds :type "Float (single-precision)"))
  (`self.UpdatePerceivedActor`))

(event `self.AIPerception.OnPerceptionUpdated`
  (params (UpdatedActors :type "Array of Actor Object Reference (by ref)"))
  (`self.PerceptionUpdated`))

(fn `ActiveAI`
  (bind _blackboard (`self.Blackboard`)
    (:`then`
      (`BlackboardComponent.SetValueAsEnum` _blackboard "StateOfBehavior" (enumliteral `/Game/01_BP/Human/Base/AI/EStateOfBehavior` "NewEnumerator4")))
    (:`else`)))

(fn `DeactiveAI`
  (bind _blackboard (`self.Blackboard`)
    (:`then`
      (`BlackboardComponent.SetValueAsEnum` _blackboard "StateOfBehavior" (enumliteral `/Game/01_BP/Human/Base/AI/EStateOfBehavior` "NewEnumerator0")))
    (:`else`)))

(fn `PerceptionUpdated`
  (if (not (`KismetSystemLibrary.IsValid` (`BlackboardComponent.GetValueAsObject` (`AIBlueprintHelperLibrary.GetBlackboard` null) "Target")))
    (for _array_element (`AIPerceptionComponent.GetCurrentlyPerceivedActors` (`self.AIPerception`) null)
      (bind _asbp_human (cast `/Game/01_BP/Human/Base/BP_Human` _array_element)) ; 만약 감지한 애가 휴먼으로 캐스팅 될 수 있다? 플레이어를 감지 했다?
      (if (!= (`/Game/01_BP/Human/Base/BP_Human.TeamID` _asbp_human) (`self.OwnerTeamID`))
        (`BlackboardComponent.SetValueAsObject` (`AIBlueprintHelperLibrary.GetBlackboard` null) "Target" _asbp_human)
        (return)))))

(fn `UpdatePerceivedActor`
  (locals (PrevTarget :type "Actor Object Reference"))
  (bind _blackboard (`self.Blackboard`)
    (:`then`
      (bind _asactor (cast `Actor` (`BlackboardComponent.GetValueAsObject` _blackboard "Target"))
        (:`then`
          _)
        (:`CastFailed`
          _))
      (set `local.PrevTarget` _asactor)
      (for _array_element (`AIPerceptionComponent.GetKnownPerceivedActors` (`self.AIPerception`) null)
        (bind _asbp_human (cast `/Game/01_BP/Human/Base/BP_Human` _array_element))
        (if (and (not (`/Game/03_Components/StateComponent.IsDeadMode` (`/Game/01_BP/Human/Base/BP_Human.StateComponent` _asbp_human))) (== _asbp_human (`local.PrevTarget`)))
          (return)))
      (`self.StopMovement`)
      (for _array_element_2 (`AIPerceptionComponent.GetKnownPerceivedActors` (`self.AIPerception`) null)
        (bind _asbp_human_2 (cast `/Game/01_BP/Human/Base/BP_Human` _array_element_2))
        (if (and (not (`/Game/03_Components/StateComponent.IsDeadMode` (`/Game/01_BP/Human/Base/BP_Human.StateComponent` _asbp_human_2))) (!= (`/Game/01_BP/Human/Base/BP_Human.TeamID` _asbp_human_2) (`self.OwnerTeamID`)))
          (`BlackboardComponent.SetValueAsObject` (`AIBlueprintHelperLibrary.GetBlackboard` null) "Target" _asbp_human_2) ; 하나도 감지를 못했을 경우, 오브젝트를 None(=Null) 처리해줌
        )))
    (:`else`)))

(fn `UserConstructionScript`)