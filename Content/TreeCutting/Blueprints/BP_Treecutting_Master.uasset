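; Master Blueprint for a choppable tree that falls and turns into logs, with its meshes assigned in the construction script.
; The first hit swaps the static tree for hidden interactive parts and starts a delayed self-destruct.
; Hits on eight destructible meshes apply radial damage and increment a counter.
; At the limit, the top falls with physics and sound, is replaced by logs spawned at its child components, then the actor is destroyed.
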(event `self.ReceiveBeginPlay`
  ;[1 1 1] Ensures no collision of interactive meshes before activated
  (`PrimitiveComponent.SetCollisionEnabled` (`self.Top`) "NoCollision")
  (`PrimitiveComponent.SetCollisionEnabled` (`self.Trunk`) "NoCollision")
  (`PrimitiveComponent.SetCollisionEnabled` (`self.DM_01`) "NoCollision")
  (`PrimitiveComponent.SetCollisionEnabled` (`self.DM_02`) "NoCollision")
  (`PrimitiveComponent.SetCollisionEnabled` (`self.DM_08`) "NoCollision")
  (`PrimitiveComponent.SetCollisionEnabled` (`self.DM_07`) "NoCollision")
  (`PrimitiveComponent.SetCollisionEnabled` (`self.DM_06`) "NoCollision")
  (`PrimitiveComponent.SetCollisionEnabled` (`self.DM_05`) "NoCollision")
  (`PrimitiveComponent.SetCollisionEnabled` (`self.DM_04`) "NoCollision")
  (`PrimitiveComponent.SetCollisionEnabled` (`self.DM_03`) "NoCollision"))

(event `self.OriginalTree.OnComponentHit`
  (params (HitComponent :type "PrimitiveComponent Object Reference") (OtherActor :type "Actor Object Reference") (OtherComp :type "PrimitiveComponent Object Reference") (NormalImpulse :type "Vector Structure") (Hit :type "HitResult Structure (by ref)"))
  (bind _top (`self.Top`))
  ;[1 1 1] Activates Interactive Tree after hit
  ;;[1 1 1] Destroys non interactive tree
  (`ActorComponent.K2_DestroyComponent` (`self.OriginalTree`))
  ;;[1 1 1] Enables collision and sets visibility of interactive parts
  (`PrimitiveComponent.SetCollisionEnabled` _top "QueryAndPhysics")
  (`PrimitiveComponent.SetCollisionEnabled` (`self.Trunk`) "QueryAndPhysics")
  (`PrimitiveComponent.SetCollisionEnabled` (`self.DM_08`) "QueryAndPhysics")
  (`PrimitiveComponent.SetCollisionEnabled` (`self.DM_07`) "QueryAndPhysics")
  (`PrimitiveComponent.SetCollisionEnabled` (`self.DM_06`) "QueryAndPhysics")
  (`PrimitiveComponent.SetCollisionEnabled` (`self.DM_05`) "QueryAndPhysics")
  (`PrimitiveComponent.SetCollisionEnabled` (`self.DM_04`) "QueryAndPhysics")
  (`PrimitiveComponent.SetCollisionEnabled` (`self.DM_03`) "QueryAndPhysics")
  (`PrimitiveComponent.SetCollisionEnabled` (`self.DM_02`) "QueryAndPhysics")
  (`PrimitiveComponent.SetCollisionEnabled` (`self.DM_01`) "QueryAndPhysics")
  (`SceneComponent.SetVisibility` _top true false)
  (`SceneComponent.SetVisibility` (`self.Trunk`) true false)
  (`SceneComponent.SetVisibility` (`self.DM_01`) true false)
  (`SceneComponent.SetVisibility` (`self.DM_02`) true false)
  (`SceneComponent.SetVisibility` (`self.DM_08`) true false)
  (`SceneComponent.SetVisibility` (`self.DM_07`) true false)
  (`SceneComponent.SetVisibility` (`self.DM_06`) true false)
  (`SceneComponent.SetVisibility` (`self.DM_05`) true false)
  (`SceneComponent.SetVisibility` (`self.DM_04`) true false)
  (`SceneComponent.SetVisibility` (`self.DM_03`) true false)
  ;[1 1 1] Destroys actor after inactivity
  (`/Engine/EditorBlueprintResources/StandardMacros.DoOnce` false
    (:`Completed`
      (`KismetSystemLibrary.Delay` (`self.DestroyActorAfterInactivity`))
      (`self.Destroy TreecuttingActor`))))

(event `Destroy TreecuttingActor`
  ;[1 1 1] Destroy the treecutting actor by event
  (`self.K2_DestroyActor`))

(event `Process_Hit_on_DM`
  (params (object :type "Actor Object Reference") (Hit :type "HitResult Structure"))
  ;[1 1 1] Processes a hit on the DM
  (`self.check_impact_object_and_apply_damage` object Hit)
  (if (not (`self.TreeIsFallen`))
    (bind _tree_can_fall (`self.CanTreeFall`))
    (if _tree_can_fall
      (`self.Let_Tree_Fall` (`.ImpactPoint` (`GameplayStatics.BreakHitResult` Hit)))
      (`KismetSystemLibrary.Delay` (`self.Duration before logs spawning`))
      (`self.spawn_Logs`)
      (`KismetSystemLibrary.Delay` (`self.Delete after time fallen`))
      (`self.Destroy TreecuttingActor`))))

(event `self.DM_01.OnComponentHit`
  (params (HitComponent :type "PrimitiveComponent Object Reference") (OtherActor :type "Actor Object Reference") (OtherComp :type "PrimitiveComponent Object Reference") (NormalImpulse :type "Vector Structure") (Hit :type "HitResult Structure (by ref)"))
  ;[1 1 1] On Component Hit DM -> Process Hit
  (`self.Process_Hit_on_DM` OtherActor Hit))

(event `self.DM_02.OnComponentHit`
  (params (HitComponent :type "PrimitiveComponent Object Reference") (OtherActor :type "Actor Object Reference") (OtherComp :type "PrimitiveComponent Object Reference") (NormalImpulse :type "Vector Structure") (Hit :type "HitResult Structure (by ref)"))
  ;[1 1 1] On Component Hit DM -> Process Hit
  (`self.Process_Hit_on_DM` OtherActor Hit))

(event `self.DM_03.OnComponentHit`
  (params (HitComponent :type "PrimitiveComponent Object Reference") (OtherActor :type "Actor Object Reference") (OtherComp :type "PrimitiveComponent Object Reference") (NormalImpulse :type "Vector Structure") (Hit :type "HitResult Structure (by ref)"))
  ;[1 1 1] On Component Hit DM -> Process Hit
  (`self.Process_Hit_on_DM` OtherActor Hit))

(event `self.DM_04.OnComponentHit`
  (params (HitComponent :type "PrimitiveComponent Object Reference") (OtherActor :type "Actor Object Reference") (OtherComp :type "PrimitiveComponent Object Reference") (NormalImpulse :type "Vector Structure") (Hit :type "HitResult Structure (by ref)"))
  ;[1 1 1] On Component Hit DM -> Process Hit
  (`self.Process_Hit_on_DM` OtherActor Hit))

(event `self.DM_05.OnComponentHit`
  (params (HitComponent :type "PrimitiveComponent Object Reference") (OtherActor :type "Actor Object Reference") (OtherComp :type "PrimitiveComponent Object Reference") (NormalImpulse :type "Vector Structure") (Hit :type "HitResult Structure (by ref)"))
  ;[1 1 1] On Component Hit DM -> Process Hit
  (`self.Process_Hit_on_DM` OtherActor Hit))

(event `self.DM_06.OnComponentHit`
  (params (HitComponent :type "PrimitiveComponent Object Reference") (OtherActor :type "Actor Object Reference") (OtherComp :type "PrimitiveComponent Object Reference") (NormalImpulse :type "Vector Structure") (Hit :type "HitResult Structure (by ref)"))
  ;[1 1 1] On Component Hit DM -> Process Hit
  (`self.Process_Hit_on_DM` OtherActor Hit))

(event `self.DM_07.OnComponentHit`
  (params (HitComponent :type "PrimitiveComponent Object Reference") (OtherActor :type "Actor Object Reference") (OtherComp :type "PrimitiveComponent Object Reference") (NormalImpulse :type "Vector Structure") (Hit :type "HitResult Structure (by ref)"))
  ;[1 1 1] On Component Hit DM -> Process Hit
  (`self.Process_Hit_on_DM` OtherActor Hit))

(event `self.DM_08.OnComponentHit`
  (params (HitComponent :type "PrimitiveComponent Object Reference") (OtherActor :type "Actor Object Reference") (OtherComp :type "PrimitiveComponent Object Reference") (NormalImpulse :type "Vector Structure") (Hit :type "HitResult Structure (by ref)"))
  ;[1 1 1] On Component Hit DM -> Process Hit
  (`self.Process_Hit_on_DM` OtherActor Hit))

(fn `CanTreeFall`
  (returns (Tree_Can_Fall :type Boolean))
  (if (`self.TreeIsFallen`)
    _
    (elif (>= (`self.count`) (`self.count_life`))
      (set `self.TreeIsFallen` true)
      (return true)
      (else
        (bind _result (`/Engine/EditorBlueprintResources/StandardMacros.IncrementInt` (`self.count`))
          (:`  `
            (set `self.count` _result)))))))

(fn `check_impact_object_and_apply_damage`
  (params (Object :type "Actor Object Reference") (Hit :type "HitResult Structure"))
  (`GameplayStatics.ApplyRadialDamage` :`BaseDamage` 4.0 :`Origin` (`.ImpactPoint` (`GameplayStatics.BreakHitResult` Hit)) :`DamageRadius` 1.0 :`DamageTypeClass` "/Script/Engine.DamageType" :`DamageCauser` null :`InstigatedByController` null))

(fn `Let_Tree_Fall`
  (params (Location :type "Vector Structure"))
  (`PrimitiveComponent.SetSimulatePhysics` (`self.Top`) true)
  (`GameplayStatics.PlaySoundAtLocation` (`self.FallingTreeSound`) Location (struct) 1.0 1.0 0.0 null null null)
  ;[1 1 1] Destroy all destructable meshes
  (for _array_element (`SceneComponent.GetChildrenComponents` (`self.Middle_Destructable`) true)
    (`ActorComponent.K2_DestroyComponent` _array_element)))

(fn `spawn_Logs`
  ;[1 1 1] Loop over child components and spawn log on location of scene components under Tree Top
  (for _array_element (`SceneComponent.GetChildrenComponents` (`self.Top`) false)
    (`|SpawnActorFromClass` (`self.Logg to spawn`) (`SceneComponent.K2_GetComponentToWorld` _array_element) "Undefined" "OverrideRootScale" null null))
  ;[1 1 1] Destroy Treetop when replaced with logs
  (`ActorComponent.K2_DestroyComponent` (`self.Top`)))

(fn `UserConstructionScript`
  (`StaticMeshComponent.SetStaticMesh` (`self.Top`) (`self.Top Mesh`))
  (`StaticMeshComponent.SetStaticMesh` (`self.Trunk`) (`self.Trunk Mesh`))
  (`StaticMeshComponent.SetStaticMesh` (`self.OriginalTree`) (`self.OriginalTreeMesh`))
  (`DestructibleComponent.SetDestructibleMesh` (`self.DM_01`) (`self.DM_Mesh_01`))
  (`DestructibleComponent.SetDestructibleMesh` (`self.DM_02`) (`self.DM_Mesh_02`))
  (`DestructibleComponent.SetDestructibleMesh` (`self.DM_03`) (`self.DM_Mesh_03`))
  (`DestructibleComponent.SetDestructibleMesh` (`self.DM_04`) (`self.DM_Mesh_04`))
  (`DestructibleComponent.SetDestructibleMesh` (`self.DM_05`) (`self.DM_Mesh_05`))
  (`DestructibleComponent.SetDestructibleMesh` (`self.DM_06`) (`self.DM_Mesh_06`))
  (`DestructibleComponent.SetDestructibleMesh` (`self.DM_07`) (`self.DM_Mesh_07`))
  (`DestructibleComponent.SetDestructibleMesh` (`self.DM_08`) (`self.DM_Mesh_08`)))