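; Boss explosion pattern actor that continuously spawns red or blue orbs at random and can set off a damaging blast.
; Spawned orbs get a back-reference to this spawner and a short lifespan.
; When the red-orb hit count passes its threshold, Tick enables the Niagara effect and sphere collision, re-setting the timer for Deactivate, which destroys the actor.
; Overlapping BP_Human actors receive knockdown damage with launch and camera shake.
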(event `self.ReceiveBeginPlay`
  (`KismetSystemLibrary.K2_SetTimerDelegate` (delegate `SpawnOrbs`) 0.1 true))

(event `SpawnOrbs`
  (bind _returnvalue (`self.GetTransform`))
  (switch `int` (`KismetMathLibrary.RandomInteger` 2)
    (:`0`
      (bind _returnvalue_2 (`|SpawnActorFromClass` "/Game/05_Weapons/Skill/Boss/Pattern/Cube/Orbs/BP_RedOrbs.BP_RedOrbs_C" _returnvalue "AlwaysSpawn" "OverrideRootScale" self null))
      (set `/Game/05_Weapons/Skill/Boss/Pattern/Cube/Orbs/BP_RedOrbs.OwnerSpawner` self _returnvalue_2)
      (`self.SetLifeSpan` _returnvalue_2 5.0))
    (:`1`
      (bind _returnvalue_3 (`|SpawnActorFromClass` "/Game/05_Weapons/Skill/Boss/Pattern/Cube/Orbs/BP_BlueOrbs.BP_BlueOrbs_C" _returnvalue "AlwaysSpawn" "OverrideRootScale" self null))
      (set `/Game/05_Weapons/Skill/Boss/Pattern/Cube/Orbs/BP_BlueOrbs.OwnerSpawner` self _returnvalue_3)
      (`self.SetLifeSpan` _returnvalue_3 5.0))))

(event `self.ReceiveTick`
  (params (DeltaSeconds :type "Float (single-precision)"))
  (bind _hitcountofredorbs (`self.HitCountOfRedOrbs`))
  (`KismetSystemLibrary.PrintString` (`KismetStringLibrary.Conv_IntToString` _hitcountofredorbs))
  (if (> _hitcountofredorbs 3)
    (`self.Activate`)
    (`KismetSystemLibrary.K2_SetTimer` self "Deactivate" 0.1)))

(event `self.Sphere.OnComponentBeginOverlap`
  (params (OverlappedComponent :type "PrimitiveComponent Object Reference") (OtherActor :type "Actor Object Reference") (OtherComp :type "PrimitiveComponent Object Reference") (OtherBodyIndex :type Integer) (bFromSweep :type Boolean) (SweepResult :type "HitResult Structure (by ref)"))
  (bind _asbp_human (cast `/Game/01_BP/Human/Base/BP_Human` OtherActor))
  (message `/Game/IDamage.Damaged` _asbp_human null self (make `/Game/05_Weapons/FHitData` 20.0 "/Game/02_Character/Montages/Common/Hit/Katana_Blade_KnockDown_Front_Damage_Montage.Katana_Blade_KnockDown_Front_Damage_Montage" 1.0 false 500.0 (struct :`Pitch` 45.0) 0.0 null "/Game/05_Weapons/OneHand/Katana/CS_Katana_Ctrl_1.CS_Katana_Ctrl_1_C" null (0.0 0.0 0.0) (0.0 0.0 0.0) false "/Game/ImproveFights_Vfx/Particles/P_WeaponWind_Hit.P_WeaponWind_Hit") (struct)))

(fn `Activate`
  (`ActorComponent.SetActive` (`self.Niagara`) true false)
  (`PrimitiveComponent.SetCollisionEnabled` (`self.Sphere`) "QueryOnly"))

(fn `Deactivate`
  (`ActorComponent.SetActive` (`self.Niagara`) false false)
  (`PrimitiveComponent.SetCollisionEnabled` (`self.Sphere`) "NoCollision")
  (`self.K2_DestroyActor`))

(fn `UserConstructionScript`)